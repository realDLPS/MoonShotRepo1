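; Bullet projectile actor that stops, flashes an impact particle effect and destroys itself when it hits certain world actors.
; Box overlap casts the other actor to terrain, meteor, large rock, hangar, Speedster or shop, ignoring already fractured meteors.
; Hits share one path: halt projectile movement, briefly pulse the particle system, then destroy after a short delay.
; A BeginPlay timer fires the same particle pulse after several seconds, without destroying the bullet.
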(event OnComponentBeginOverlap(Box)
  (params (OverlappedComponent :type Primitive%20Component%20Object%20Reference) (OtherActor :type Actor%20Object%20Reference) (OtherComp :type Primitive%20Component%20Object%20Reference) (OtherBodyIndex :type Integer) (bFromSweep :type Boolean) (SweepResult :type Hit%20Result%20Structure%20%28by%20ref%29))
  (bind _particlesystem (Variables|Default|GetParticleSystem))
  (Utilities|FlowControl|Sequence
    (:then_0
      (Utilities|Casting|CastToTerrain OtherActor)
      (Components|Movement|StopMovementImmediately (Variables|Default|GetProjectileMovement) :!label _label)
      (Utilities|FlowControl|Sequence
        (:then_0
          (Components|Activation|Activate _particlesystem false)
          (Utilities|FlowControl|Delay 0.2)
          (Components|Activation|Deactivate _particlesystem))
        (:then_1
          (Utilities|FlowControl|Delay 0.2)
          (Actor|DestroyActor))))
    (:then_1
      (bind _asmeteor (Utilities|Casting|CastToMeteor OtherActor))
      (if (not (Variables|/Game/HideThis/Meteor.Meteor_C|GetHasFractured _asmeteor))
        (goto _label)))
    (:then_2
      (Utilities|Casting|CastToRockLargeA OtherActor)
      (goto _label))
    (:then_3
      (Utilities|Casting|CastToHangarA OtherActor)
      (goto _label))
    (:then_4
      (Utilities|Casting|CastToSpeedster OtherActor)
      (goto _label))
    (:then_5
      (Utilities|Casting|CastToShop OtherActor)
      (goto _label))))

(event EventBeginPlay
  (bind _particlesystem (Variables|Default|GetParticleSystem))
  (Utilities|FlowControl|Delay 1.0)
  (Utilities|FlowControl|Delay 5.0)
  (Components|Activation|Activate _particlesystem false)
  (Utilities|FlowControl|Delay 0.2)
  (Components|Activation|Deactivate _particlesystem))

(event Collision|EventActorBeginOverlap
  (params (OtherActor :type Actor%20Object%20Reference)))

(event EventTick
  (params (DeltaSeconds :type Float%20%28single-precision%29)))

(fn ConstructionScript)