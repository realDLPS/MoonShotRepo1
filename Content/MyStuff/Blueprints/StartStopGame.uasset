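; Trigger actor that lets the player start and stop meteorite spawning while standing inside its box.
; Entering the box as the ThirdPersonCharacter sets an in-trigger flag and shows a StartStopGameWidget; leaving clears the flag and removes that widget.
; While the flag is set, the Start/Stop Game input runs a FlipFlop that alternately turns ShouldMeteoritesSpawn on and off on the player character.
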(event OnComponentBeginOverlap(Box)
  (params (OverlappedComponent :type Primitive%20Component%20Object%20Reference) (OtherActor :type Actor%20Object%20Reference) (OtherComp :type Primitive%20Component%20Object%20Reference) (OtherBodyIndex :type Integer) (bFromSweep :type Boolean) (SweepResult :type Hit%20Result%20Structure%20%28by%20ref%29))
  (Utilities|Casting|CastToThirdPersonCharacter OtherActor)
  (Variables|Default|SetIsInTrigger true)
  (bind _returnvalue (UserInterface|CreateWidget "/Game/MyStuff/UI/StartStopGameWidget.StartStopGameWidget_C"))
  (UserInterface|Viewport|AddtoViewport _returnvalue 0))

(event OnComponentEndOverlap(Box)
  (params (OverlappedComponent :type Primitive%20Component%20Object%20Reference) (OtherActor :type Actor%20Object%20Reference) (OtherComp :type Primitive%20Component%20Object%20Reference) (OtherBodyIndex :type Integer))
  (Utilities|Casting|CastToThirdPersonCharacter OtherActor)
  (Variables|Default|SetIsInTrigger false)
  (bind _foundwidgets (Widget|GetAllWidgetsOfClass "/Game/MyStuff/UI/StartStopGameWidget.StartStopGameWidget_C" true))
  (Widget|RemovefromParent _foundwidgets))

(event EventBeginPlay)

(event Collision|EventActorBeginOverlap
  (params (OtherActor :type Actor%20Object%20Reference)))

(event EventTick
  (params (DeltaSeconds :type Float%20%28single-precision%29)))

(event Input|ActionEvents|InputActionStart/StopGame
  (params (Key :type Key%20Structure :default "None"))
  (bind _returnvalue (Game|GetPlayerCharacter 0))
  (:Pressed
    (if (Variables|Default|GetIsInTrigger)
      (Utilities|FlowControl|FlipFlop
        (:A
          (bind _asthird_person_character (Utilities|Casting|CastToThirdPersonCharacter _returnvalue))
          (Variables|/Game/HideThis/ThirdPersonBP/Blueprints/ThirdPersonCharacter.ThirdPersonCharacter_C|SetShouldMeteoritesSpawn _asthird_person_character true))
        (:B
          (bind _asthird_person_character_2 (Utilities|Casting|CastToThirdPersonCharacter _returnvalue))
          (Variables|/Game/HideThis/ThirdPersonBP/Blueprints/ThirdPersonCharacter.ThirdPersonCharacter_C|SetShouldMeteoritesSpawn _asthird_person_character_2 false))))))

(fn ConstructionScript)