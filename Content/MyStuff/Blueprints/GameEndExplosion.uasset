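; GameEndExplosion is an actor that plays the game-over explosion and resets the player's progress when the ThirdPersonCharacter dies.
; From BeginPlay it polls the character's Health once per second through a self-looping Delay.
; At zero or below it resets the character's score, cash, stats, upgrade costs and meteor spawning, then activates three fire particle effects and deactivates them three seconds later.
; The check does not restart after firing.
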(event EventBeginPlay
  (bind _outactors (Actor|GetAllActorsOfClass "/Game/HideThis/ThirdPersonBP/Blueprints/ThirdPersonCharacter.ThirdPersonCharacter_C" :!label _label))
  (if (<= (Variables|/Game/HideThis/ThirdPersonBP/Blueprints/ThirdPersonCharacter.ThirdPersonCharacter_C|GetHealth (Utilities|Array|Get(acopy) _outactors)) 0)
    (bind _outactors_2 (Actor|GetAllActorsOfClass "/Game/HideThis/ThirdPersonBP/Blueprints/ThirdPersonCharacter.ThirdPersonCharacter_C"))
    (Variables|/Game/HideThis/ThirdPersonBP/Blueprints/ThirdPersonCharacter.ThirdPersonCharacter_C|SetScore (Utilities|Array|Get(acopy) _outactors_2) 0)
    (Variables|/Game/HideThis/ThirdPersonBP/Blueprints/ThirdPersonCharacter.ThirdPersonCharacter_C|SetCash (Utilities|Array|Get(acopy) _outactors_2) 0)
    (Variables|/Game/HideThis/ThirdPersonBP/Blueprints/ThirdPersonCharacter.ThirdPersonCharacter_C|SetFirerate (Utilities|Array|Get(acopy) _outactors_2) 1.0)
    (Variables|/Game/HideThis/ThirdPersonBP/Blueprints/ThirdPersonCharacter.ThirdPersonCharacter_C|SetCashAmountGotten (Utilities|Array|Get(acopy) _outactors_2) 10)
    (Variables|/Game/HideThis/ThirdPersonBP/Blueprints/ThirdPersonCharacter.ThirdPersonCharacter_C|SetHealth (Utilities|Array|Get(acopy) _outactors_2) 10)
    (Variables|/Game/HideThis/ThirdPersonBP/Blueprints/ThirdPersonCharacter.ThirdPersonCharacter_C|SetMaxAmmo (Utilities|Array|Get(acopy) _outactors_2) 5)
    (Variables|/Game/HideThis/ThirdPersonBP/Blueprints/ThirdPersonCharacter.ThirdPersonCharacter_C|SetAmmo (Utilities|Array|Get(acopy) _outactors_2) 5)
    (Variables|/Game/HideThis/ThirdPersonBP/Blueprints/ThirdPersonCharacter.ThirdPersonCharacter_C|SetReloadSpeed (Utilities|Array|Get(acopy) _outactors_2) 2.0)
    (Variables|/Game/HideThis/ThirdPersonBP/Blueprints/ThirdPersonCharacter.ThirdPersonCharacter_C|SetFirerateCost (Utilities|Array|Get(acopy) _outactors_2) 10)
    (Variables|/Game/HideThis/ThirdPersonBP/Blueprints/ThirdPersonCharacter.ThirdPersonCharacter_C|SetCashMultiplierCost (Utilities|Array|Get(acopy) _outactors_2) 100)
    (Variables|/Game/HideThis/ThirdPersonBP/Blueprints/ThirdPersonCharacter.ThirdPersonCharacter_C|SetHealthCost (Utilities|Array|Get(acopy) _outactors_2) 25)
    (Variables|/Game/HideThis/ThirdPersonBP/Blueprints/ThirdPersonCharacter.ThirdPersonCharacter_C|SetMaxAmmoCost (Utilities|Array|Get(acopy) _outactors_2) 25)
    (Variables|/Game/HideThis/ThirdPersonBP/Blueprints/ThirdPersonCharacter.ThirdPersonCharacter_C|SetReloadSpeedCost (Utilities|Array|Get(acopy) _outactors_2) 10)
    (Variables|/Game/HideThis/ThirdPersonBP/Blueprints/ThirdPersonCharacter.ThirdPersonCharacter_C|SetMeteorSpawnRate (Utilities|Array|Get(acopy) _outactors_2) 6.0)
    (Variables|/Game/HideThis/ThirdPersonBP/Blueprints/ThirdPersonCharacter.ThirdPersonCharacter_C|SetShouldMeteoritesSpawn (Utilities|Array|Get(acopy) _outactors_2) false)
    (Components|Activation|Activate (Variables|Default|GetFire_Exp_00) false)
    (Components|Activation|Activate (Variables|Default|GetFire_Exp_01) false)
    (Components|Activation|Activate (Variables|Default|GetFire_Exp_03) false)
    (Utilities|FlowControl|Delay 3.0)
    (Components|Activation|Deactivate (Variables|Default|GetFire_Exp_00))
    (Components|Activation|Deactivate (Variables|Default|GetFire_Exp_01))
    (Components|Activation|Deactivate (Variables|Default|GetFire_Exp_03))
    (else
      (Utilities|FlowControl|Delay 1.0)
      (goto _label))))

(event Collision|EventActorBeginOverlap
  (params (OtherActor :type Actor%20Object%20Reference)))

(event EventTick
  (params (DeltaSeconds :type Float%20%28single-precision%29)))

(fn ConstructionScript)